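; Fairy particle actor that follows an AI_BP character and removes itself when an AI dies.
; Each Tick it searches all AI_BP actors and destroys itself once if any of them has IsDead set.
; It also re-attaches itself every frame to each AI_BP's ParticleDust socket in turn, so it ends up snapped to the last one found.
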(event `self.ReceiveTick`
  (params (DeltaSeconds :type "Float (single-precision)"))
  (`|ExecutionSequence`
    (:`then_0`
      (bind _outactors (`GameplayStatics.GetAllActorsOfClass` "/Game/AI/AI_BP.AI_BP_C"))
      (for _array_element _outactors
        (bind _asai_bp (cast `/Game/AI/AI_BP` _array_element))
        (if (`/Game/AI/AI_BP.IsDead` _asai_bp)
          (`/Engine/EditorBlueprintResources/StandardMacros.DoOnce` false
            (:`Completed`
              (`self.K2_DestroyActor`))))))
    (:`then_1`
      (bind _outactors_2 (`GameplayStatics.GetAllActorsOfClass` "/Game/AI/AI_BP.AI_BP_C"))
      (for _array_element_2 _outactors_2
        (bind _asai_bp_2 (cast `/Game/AI/AI_BP` _array_element_2))
        (`self.K2_AttachToActor` _asai_bp_2 "ParticleDust" "SnapToTarget" "SnapToTarget" "KeepRelative")))))

(fn `UserConstructionScript`)