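; AI enemy pawn that roams the navmesh after landing, chases the player and reports kills to FirstPersonGameMode on death.
; PawnSensing sightings or overlaps start ChasePlayer, which repeats move-and-damage while the player lives.
; Overlapping the player damages both sides; depleted health triggers blood, squish sound and destruction.
; AttachParticle snaps every FairyParticle_BP actor in the level to its ParticleDust socket.
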(event `Attach Particle`
  (bind _outactors (`GameplayStatics.GetAllActorsOfClass` "/Game/AI/FairyParticle_BP.FairyParticle_BP_C"))
  (for _array_element _outactors
    (bind _asfairy_particle_bp (cast `/Game/AI/FairyParticle_BP` _array_element))
    (`self.K2_AttachToActor` _asfairy_particle_bp self "ParticleDust" "SnapToTarget" "SnapToTarget" "KeepRelative" true)))

(event `self.OnLanded`
  (params (Hit :type "HitResult Structure (by ref)"))
  (`|AIMoveTo` self (`NavigationSystem.K2_GetRandomLocationInNavigableRadius` (`self.K2_GetActorLocation`) 500.0) :!label _label
    (:`OnSuccess`
      (`KismetSystemLibrary.Delay` 1.0)
      (`self.Roam`))))

(event `Roam`
  (goto _label))

(event `Death`
  (bind _capsulecomponent (`self.CapsuleComponent`))
  (`GameplayStatics.SpawnEmitterAttached` "/Game/Particles/Blood_P.Blood_P" _capsulecomponent "None" (0.0 0.0 80.0) (struct) (0.3 0.3 0.3) "SnapToTargetIncludingScale")
  (`GameplayStatics.PlaySoundAtLocation` "/Game/Audio/squish.squish" (`SceneComponent.K2_GetComponentLocation` _capsulecomponent))
  (bind _asfirst_person_game_mode (cast `/Game/FirstPersonBP/Blueprints/FirstPersonGameMode` (`GameplayStatics.GetGameMode`)))
  (`/Game/FirstPersonBP/Blueprints/FirstPersonGameMode.Add Kills` _asfirst_person_game_mode (`self.Kills`))
  (`KismetSystemLibrary.Delay` 0.2)
  (set `self.IsDead` true)
  (`self.K2_DestroyActor`))

(event `self.ReceiveAnyDamage`
  (params (Damage :type "Float (single-precision)") (DamageType :type "DamageType Object Reference") (InstigatedBy :type "Controller Object Reference") (DamageCauser :type "Actor Object Reference"))
  (bind _output_get (set `self.Health` (- (`self.Health`) (`KismetMathLibrary.FTrunc` Damage))))
  (if (<= _output_get 0)
    (`self.Death`)))

(event `ChasePlayer`
  (params (`Player to Chase` :type "Pawn Object Reference"))
  (bind _asfirst_person_character (cast `/Game/FirstPersonBP/Blueprints/FirstPersonCharacter` (`GameplayStatics.GetPlayerCharacter` 0)))
  (if (<= (`/Game/FirstPersonBP/Blueprints/FirstPersonCharacter.Health` _asfirst_person_character) 0.0)
    _
    (elif (`PawnSensingComponent.bEnableSensingUpdates` (`self.PawnSensing`))
      (`|AIMoveTo` self (0.0 0.0 0.0) `Player to Chase`
        (:`OnSuccess`
          (`GameplayStatics.ApplyDamage` _asfirst_person_character 10.0 null self)
          (`KismetSystemLibrary.Delay` 1.0)
          (`self.ChasePlayer` `Player to Chase`))))))

(event `self.ReceiveActorBeginOverlap`
  (params (OtherActor :type "Actor Object Reference"))
  (bind _asfirst_person_character (cast `/Game/FirstPersonBP/Blueprints/FirstPersonCharacter` OtherActor))
  (`GameplayStatics.ApplyDamage` _asfirst_person_character 10.0 (`AIBlueprintHelperLibrary.GetAIController` null) self)
  (`GameplayStatics.ApplyDamage` self 30.0)
  (`self.ChasePlayer` _asfirst_person_character))

(event `self.PawnSensing.OnSeePawn`
  (params (Pawn :type "Pawn Object Reference"))
  (bind _asfirst_person_character (cast `/Game/FirstPersonBP/Blueprints/FirstPersonCharacter` Pawn))
  (`self.ChasePlayer` _asfirst_person_character))

(fn `UserConstructionScript`)